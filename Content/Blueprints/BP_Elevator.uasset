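; Elevator actor that the player calls with an interact prompt, moving its cabin along a spline.
; A trigger box registers it as the player's interactable, and Interact toggles a timeline driving the cabin forward or back.
; When the player leaves a second box while IsUp is set, it reverses after a short delay.
; A dynamic-material sphere starts red and is recolored red or green on Interact from IsUp's pre-toggle value.
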(event `self.ReceiveBeginPlay`
  (bind _asbp_player_character (cast `/Game/Blueprints/BP_PlayerCharacter` (`GameplayStatics.GetPlayerPawn` 0)))
  (set `self.Player` _asbp_player_character))

(event `self.BoxTrigger.OnComponentBeginOverlap`
  (params (OverlappedComponent :type "PrimitiveComponent Object Reference") (OtherActor :type "Actor Object Reference") (OtherComp :type "PrimitiveComponent Object Reference") (OtherBodyIndex :type Integer) (bFromSweep :type Boolean) (SweepResult :type "HitResult Structure (by ref)"))
  (bind _player (`self.Player`))
  (if (== OtherActor _player)
    (set `/Game/Blueprints/BP_PlayerCharacter.CanInteractwE` true _player)
    (set `/Game/Blueprints/BP_PlayerCharacter.E_Interuptor` self (`self.Player`))))

(event `self.BoxTrigger.OnComponentEndOverlap`
  (params (OverlappedComponent :type "PrimitiveComponent Object Reference") (OtherActor :type "Actor Object Reference") (OtherComp :type "PrimitiveComponent Object Reference") (OtherBodyIndex :type Integer))
  (bind _player (`self.Player`))
  (if (== OtherActor _player)
    (set `/Game/Blueprints/BP_PlayerCharacter.CanInteractwE` false _player)
    (set `/Game/Blueprints/BP_PlayerCharacter.E_Interuptor` null (`self.Player`))))

(event `StartMovement`
  (set `self.IsUp` true)
  (bind (_direction _alpha) (`Timeline|Timeline_0` :!label _label)
    (:`Update`
      (`SceneComponent.K2_SetRelativeLocation` (`self.Cabine`) (`SplineComponent.GetLocationAtTime` (`self.Spline`) _alpha "Local" false) false false))))

(event `ReverseMovement`
  (set `self.IsUp` false)
  (goto _label :!via `Reverse`))

(event `self.Box.OnComponentEndOverlap`
  (params (OverlappedComponent :type "PrimitiveComponent Object Reference") (OtherActor :type "Actor Object Reference") (OtherComp :type "PrimitiveComponent Object Reference") (OtherBodyIndex :type Integer))
  (if (== OtherActor (`self.Player`))
    (if (`self.IsUp`)
      (`KismetSystemLibrary.Delay` 3.0)
      (`self.ReverseMovement`))))

(fn `Interact`
  (bind _materialref (`self.MaterialRef`))
  (bind _isup (`self.IsUp`))
  (bind _returnvalue (select `bool` _isup :`false` (struct :`R` 1.0 :`A` 1.0) :`true` (struct :`G` 1.0 :`A` 1.0) :!type "LinearColor Structure"))
  (if _isup
    (`MaterialInstanceDynamic.SetVectorParameterValue` _materialref "Color" _returnvalue)
    (`self.ReverseMovement`)
    (else
      (`MaterialInstanceDynamic.SetVectorParameterValue` _materialref "Color" _returnvalue)
      (`self.StartMovement`))))

(fn `UserConstructionScript`
  (bind _returnvalue (`PrimitiveComponent.CreateDynamicMaterialInstance` (`self.Sphere`) 0 "/Game/Marerials/G_Red.G_Red" "None"))
  (bind _output_get (set `self.MaterialRef` _returnvalue))
  (`MaterialInstanceDynamic.SetVectorParameterValue` _output_get "Color" (struct :`R` 1.0 :`A` 1.0)))