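; BP_PressPlate is a pressure plate that sinks when a Pusher-tagged actor overlaps its trigger and rises when one leaves.
; A timeline moves the Cube mesh along a spline, reversing on exit.
; Both transitions send ActiveMessage to a linked ObjectToActive.
; It also registers itself on the cached player and one movable cube, the last found at BeginPlay, regardless of which actor overlapped.
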(event `self.ReceiveBeginPlay`
  (bind _asbp_player_character (cast `/Game/Blueprints/BP_PlayerCharacter` (`GameplayStatics.GetPlayerPawn` 0)))
  (set `self.Player` _asbp_player_character)
  (bind _outactors (`GameplayStatics.GetAllActorsOfClass` "/Game/Blueprints/BP_MovableCube.BP_MovableCube_C"))
  (for _array_element _outactors
    (bind _asbp_movable_cube (cast `/Game/Blueprints/BP_MovableCube` _array_element))
    (set `self.Box` _asbp_movable_cube)))

(event `self.BoxTrigger.OnComponentBeginOverlap`
  (params (OverlappedComponent :type "PrimitiveComponent Object Reference") (OtherActor :type "Actor Object Reference") (OtherComp :type "PrimitiveComponent Object Reference") (OtherBodyIndex :type Integer) (bFromSweep :type Boolean) (SweepResult :type "HitResult Structure (by ref)"))
  (if (`self.ActorHasTag` OtherActor "Pusher")
    (set `/Game/Blueprints/BP_PlayerCharacter.PressPlate` self (`self.Player`))
    (set `/Game/Blueprints/BP_MovableCube.PressPlate` self (`self.Box`))
    (`self.GoDown`)
    (`self.Interact`)))

(event `self.BoxTrigger.OnComponentEndOverlap`
  (params (OverlappedComponent :type "PrimitiveComponent Object Reference") (OtherActor :type "Actor Object Reference") (OtherComp :type "PrimitiveComponent Object Reference") (OtherBodyIndex :type Integer))
  (if (`self.ActorHasTag` OtherActor "Pusher")
    (set `/Game/Blueprints/BP_PlayerCharacter.PressPlate` self (`self.Player`))
    (set `/Game/Blueprints/BP_MovableCube.PressPlate` self (`self.Box`))
    (`self.GoUp`)
    (`self.Interact`)))

(event `GoDown`
  (bind (_direction _alpha) (`Timeline|Timeline_0` :!label _label)
    (:`Update`
      (`SceneComponent.K2_SetRelativeLocation` (`self.Cube`) (`SplineComponent.GetLocationAtTime` (`self.Spline`) _alpha "Local" false) false false))))

(event `GoUp`
  (goto _label :!via `Reverse`))

(fn `Interact`
  (bind _objecttoactive (`self.ObjectToActive`)
    (:`then`
      (message `/Game/Blueprints/BPI_Interuptor.Active` _objecttoactive))
    (:`else`)))

(fn `UserConstructionScript`)