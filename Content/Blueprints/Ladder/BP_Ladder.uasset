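; Portable, physics-driven ladder that the player carries on back or in hands, or climbs when grounded.
; Builds stacked mesh chunks, resizing collision, trigger and climb spline to match.
; State changes set physics, collision and folded or unfolded size; on the ground, a timer tints it green when slope allows climbing, red otherwise.
; Trigger overlap snaps the player to the spline start and enables climbing, rearming shortly after they leave.
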(event `self.ReceiveBeginPlay`
  ;[1 1 1] Set the starting ladder state
  (`self.SetLadderState` (`self.LadderState`)))

(event `self.Trigger.OnComponentBeginOverlap`
  (params (OverlappedComponent :type "PrimitiveComponent Object Reference") (OtherActor :type "Actor Object Reference") (OtherComp :type "PrimitiveComponent Object Reference") (OtherBodyIndex :type Integer) (bFromSweep :type Boolean) (SweepResult :type "HitResult Structure (by ref)"))
  ;[1 1 1] Set the player on ladder
  (if (`self.IsOnTheGround`)
    (bind _asbp_player_character (cast `/Game/Blueprints/BP_PlayerCharacter` OtherActor))
    (if (`self.CanClimb`)
      (bind _output_get (set `self.Player` _asbp_player_character))
      (set `/Game/Blueprints/BP_PlayerCharacter.CanClimb` true _output_get)
      (`self.K2_SetActorLocation` (`self.Player`) (`SplineComponent.GetLocationAtSplinePoint` (`self.Spline`) 0 "World") false false)
      ;[1 1 1] Disable trigger
      (`PrimitiveComponent.SetCollisionEnabled` (`self.Trigger`) "NoCollision"))))

(event `OnPlayerLeave`
  ;[1 1 1] Enable trigger
  (`KismetSystemLibrary.Delay` 1.0)
  (`PrimitiveComponent.SetCollisionEnabled` (`self.Trigger`) "QueryAndPhysics"))

(fn `CanClimb`
  (returns (Value :type Boolean))
  (bind _outslopepitchdegreeangle (`KismetMathLibrary.GetSlopeDegreeAngles` (`self.GetActorRightVector`) (`KismetMathLibrary.MakeVector` 0.0 0.0 1.0) (`self.GetActorUpVector`)))
  ;[1 1 1] Check if the player can climb
  (return (and (`|EnumEquality` (`self.LadderState`) "NewEnumerator2") (and (> _outslopepitchdegreeangle -45.0) (< _outslopepitchdegreeangle 45.0)))))

(fn `ClearLaderMesh`
  ;[1 1 1] Clear the ladder mesh
  (if (!= (`KismetArrayLibrary.Array_Length` (`self.LadderMeshes`)) 0)
    (for _array_element (`self.LadderMeshes`)
      (`ActorComponent.K2_DestroyComponent` _array_element))
    (`KismetArrayLibrary.Array_Clear` (`self.LadderMeshes`))))

(fn `ConstructLadder`
  (params (AddTop :type Boolean :default true))
  (bind _ladderuniformscale (`self.LadderUniformScale`))
  (bind _ladderuniformscale_2 (`self.LadderUniformScale`))
  (`|ExecutionSequence`
    (:`then_0`
      ;[1 1 1] Create ladder chunks
      (for _index (range (`self.NbLadderChunk`))
        (bind _returnvalue (`AddComponent|NODE_AddStaticMeshComponent-0` :`bManualAttachment` true :`RelativeTransform` (`KismetMathLibrary.MakeTransform` (`KismetMathLibrary.MakeVector` 0.0 0.0 (+ (* _index (`self.ChunkOffset`)) (`self.TopOffset`) (`self.ZOffset`))) (struct :`Yaw` 90.0) (`KismetMathLibrary.MakeVector` _ladderuniformscale_2 _ladderuniformscale_2 _ladderuniformscale_2))))
        ;[1 1 1] Attach the ladder and set a material
        (`SceneComponent.K2_AttachToComponent` _returnvalue (`self.Root`) "None" "KeepRelative" "KeepRelative" "KeepRelative" true)
        (`PrimitiveComponent.SetMaterial` _returnvalue 0 (`self.MaterialRef`))
        (`KismetArrayLibrary.Array_AddUnique` (`self.LadderMeshes`) _returnvalue)))
    (:`then_1`
      ;[1 1 1] Create ladder top
      (if AddTop
        (bind _returnvalue_2 (`AddComponent|NODE_AddStaticMeshComponent-2` :`bManualAttachment` true :`RelativeTransform` (`KismetMathLibrary.MakeTransform` (`KismetMathLibrary.MakeVector` 0.0 0.0 (+ (* (`self.NbLadderChunk`) (`self.ChunkOffset`)) (`self.TopOffset`) (`self.ZOffset`))) (struct :`Yaw` 90.0) (`KismetMathLibrary.MakeVector` _ladderuniformscale _ladderuniformscale _ladderuniformscale))))
        ;[1 1 1] Attach the ladder and set a material
        (`SceneComponent.K2_AttachToComponent` _returnvalue_2 (`self.Root`) "None" "KeepRelative" "KeepRelative" "KeepRelative" true)
        (`PrimitiveComponent.SetMaterial` _returnvalue_2 0 (`self.MaterialRef`))
        (`KismetArrayLibrary.Array_AddUnique` (`self.LadderMeshes`) _returnvalue_2)))))

(fn `IsOnTheGround`
  (returns (Value :type Boolean))
  ;[1 1 1] If the ladder is on the ground
  (return (`|EnumEquality` (`self.LadderState`) "NewEnumerator2")))

(fn `SetLadderSize`
  (params (Size :type Integer :default 1))
  ;[1 1 1] Set the ladder size
  (set `self.NbLadderChunk` (`KismetMathLibrary.Clamp` Size 1 100))
  (`self.ClearLaderMesh`)
  (`self.ConstructLadder` true)
  (`self.UpdateCollisionSize`)
  (`self.UpdateSpline`))

(fn `SetLadderState`
  (params (State :type "/Game/Blueprints/Ladder/E_LadderState Enum" :default "NewEnumerator0"))
  (bind _root (`self.Root`))
  (bind _root_2 (`self.Root`))
  ;[1 1 1] Set ladder state and update collisions
  (bind _output_get (set `self.LadderState` State))
  (switch `/Game/Blueprints/Ladder/E_LadderState` _output_get
    (:`NewEnumerator0`
      (`PrimitiveComponent.SetSimulatePhysics` _root_2 false)
      (`PrimitiveComponent.SetCollisionEnabled` _root_2 "NoCollision")
      (`PrimitiveComponent.SetCollisionEnabled` (`self.Collision`) "NoCollision")
      (`self.SetLadderSize` (`self.FoldedSize`))
      ;[1 1 1] Stop the timer if it's running
      (if (`KismetSystemLibrary.K2_IsTimerActiveHandle` (`self.LadderColorTimerHandle`)) :!label _label
        (`KismetSystemLibrary.K2_ClearAndInvalidateTimerHandle` (`self.LadderColorTimerHandle`)))
      (`MaterialInstanceDynamic.SetVectorParameterValue` (`self.MaterialRef`) "Color" (struct :`R` 1.0 :`A` 1.0)))
    (:`NewEnumerator1`
      (`PrimitiveComponent.SetSimulatePhysics` (`self.Root`) true)
      (`PrimitiveComponent.SetCollisionEnabled` (`self.Collision`) "QueryAndPhysics")
      (`PrimitiveComponent.SetCollisionEnabled` (`self.Root`) "QueryAndPhysics")
      (`self.SetLadderSize` (`self.UnfoldedSize`))
      (goto _label))
    (:`NewEnumerator2`
      (`PrimitiveComponent.SetSimulatePhysics` _root true)
      (`PrimitiveComponent.SetCollisionEnabled` _root "QueryAndPhysics")
      (`PrimitiveComponent.SetCollisionEnabled` (`self.Collision`) "QueryAndPhysics")
      (`PrimitiveComponent.SetCollisionResponseToAllChannels` (`self.Collision`) "ECR_Block")
      (`PrimitiveComponent.SetCollisionResponseToAllChannels` (`self.Root`) "ECR_Block")
      (`self.SetLadderSize` (`self.UnfoldedSize`))
      ;[1 1 1] Start the color timer
      (bind _returnvalue (`KismetSystemLibrary.K2_SetTimer` self "UpdateLadderColor" 0.1 true))
      (set `self.LadderColorTimerHandle` _returnvalue))))

(fn `UpdateCollisionSize`
  (bind _chunkoffset (`self.ChunkOffset`))
  (bind _returnvalue (* (`self.NbLadderChunk`) (* (`self.ChunkOffset`) 0.5)))
  (bind _returnvalue_2 (* (- (* (`self.NbLadderChunk`) _chunkoffset) _chunkoffset) 0.5))
  ;[1 1 1] Compute collision height
  (`|ExecutionSequence`
    (:`then_0`
      (`BoxComponent.SetBoxExtent` (`self.Collision`) (`KismetMathLibrary.MakeVector` 5.0 54.0 _returnvalue) true)
      ;[1 1 1] Compute collision Z
      (`SceneComponent.K2_SetRelativeLocation` (`self.Collision`) (`KismetMathLibrary.MakeVector` 0.0 0.0 _returnvalue_2) false false))
    (:`then_1`
      ;[1 1 1] Update the trigger
      (`BoxComponent.SetBoxExtent` (`self.Trigger`) (`KismetMathLibrary.MakeVector` 20.0 54.0 _returnvalue) true)
      (`SceneComponent.K2_SetRelativeLocation` (`self.Trigger`) (`KismetMathLibrary.MakeVector` -25.0 0.0 _returnvalue_2) false false))))

(fn `UpdateLadderColor`
  ;[1 1 1] Update ladder color
  (`MaterialInstanceDynamic.SetVectorParameterValue` (`self.MaterialRef`) "Color" (select `bool` (`self.CanClimb`) :`false` (struct :`R` 1.0 :`A` 1.0) :`true` (struct :`G` 1.0 :`A` 1.0) :!type "LinearColor Structure")))

(fn `UpdateSpline`
  ;[1 1 1] Update the last spline point
  (`SplineComponent.SetLocationAtSplinePoint` (`self.Spline`) 1 (`KismetMathLibrary.MakeVector` 0.0 0.0 (* (`self.NbLadderChunk`) (`self.ChunkOffset`))) "Local" true))

(fn `UserConstructionScript`
  ;[1 1 1] Create a material instance
  (bind _returnvalue (`KismetMaterialLibrary.CreateDynamicMaterialInstance` "/Game/Meshes/Ladder/MI_Ladder.MI_Ladder"))
  (set `self.MaterialRef` _returnvalue)
  ;[1 1 1] Construct the ladder
  (`self.ConstructLadder` true)
  (`self.UpdateCollisionSize`)
  (`self.UpdateSpline`))