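; BP_Cabine is a one-way ride cabin that carries the player along a spline once they step into its trigger box.
; The overlap plays a timeline that rolls the left door shut, then a second timeline moves the cabin along the spline in local space.
; On arrival it disables the trigger's collision, reverses the left door and opens the right door.
; The Interact function is empty.
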(event `self.ReceiveBeginPlay`
  (bind _asbp_player_character (cast `/Game/Blueprints/BP_PlayerCharacter` (`GameplayStatics.GetPlayerPawn` 0)))
  (set `self.Player` _asbp_player_character))

(event `ActiveCabine`
  (bind _leftdoor (`self.LeftDoor`))
  (bind (_direction _speed) (`Timeline|Timeline_door` :!label _label)
    (:`Update`
      (`SceneComponent.K2_SetRelativeRotation` _leftdoor (`KismetMathLibrary.MakeRotator` _speed (.pitch (`SceneComponent.RelativeRotation` _leftdoor)) (.yaw (`SceneComponent.RelativeRotation` _leftdoor))) false false))
    (:`Finished`
      (bind (_direction_2 _alpha) (`Timeline|Timeline_0`)
        (:`Update`
          (`SceneComponent.K2_SetRelativeLocation` (`self.Cabine`) (`SplineComponent.GetLocationAtTime` (`self.Spline`) _alpha "Local" false) false false))
        (:`Finished`
          (`PrimitiveComponent.SetCollisionEnabled` (`self.Box`) "NoCollision")
          (`self.OpenLeftDoor`)
          (`self.OpenRightDoor`))))))

(event `OpenLeftDoor`
  (goto _label :!via `Reverse`))

(event `OpenRightDoor`
  (bind _rightdoor (`self.RightDoor`))
  (bind (_direction _angle) (`Timeline|Timeline_rDoor`)
    (:`Update`
      (`SceneComponent.K2_SetRelativeRotation` _rightdoor (`KismetMathLibrary.MakeRotator` _angle (.pitch (`SceneComponent.RelativeRotation` _rightdoor)) (.yaw (`SceneComponent.RelativeRotation` _rightdoor))) false false))))

(event `self.Box.OnComponentBeginOverlap`
  (params (OverlappedComponent :type "PrimitiveComponent Object Reference") (OtherActor :type "Actor Object Reference") (OtherComp :type "PrimitiveComponent Object Reference") (OtherBodyIndex :type Integer) (bFromSweep :type Boolean) (SweepResult :type "HitResult Structure (by ref)"))
  (if (== OtherActor (`self.Player`))
    (`self.ActiveCabine`)))

(fn `Interact`)

(fn `UserConstructionScript`)