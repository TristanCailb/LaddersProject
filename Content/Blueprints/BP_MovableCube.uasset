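; BP_MovableCube is a cube actor that tells the player character which side it is on for pushing and shows a widget nearby.
; Left and Right overlap volumes set the player's LeftPush flag to true or false; no movement logic lives here.
; Entering the Box volume creates a Caisse widget, and leaving removes the first one found by a class search rather than a stored reference.
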(event `self.ReceiveBeginPlay`
  (bind _asbp_player_character (cast `/Game/Blueprints/BP_PlayerCharacter` (`GameplayStatics.GetPlayerPawn` 0)))
  (set `self.Player` _asbp_player_character))

(event `self.Left.OnComponentBeginOverlap`
  (params (OverlappedComponent :type "PrimitiveComponent Object Reference") (OtherActor :type "Actor Object Reference") (OtherComp :type "PrimitiveComponent Object Reference") (OtherBodyIndex :type Integer) (bFromSweep :type Boolean) (SweepResult :type "HitResult Structure (by ref)"))
  (bind _player (`self.Player`))
  (if (== OtherActor _player)
    (set `/Game/Blueprints/BP_PlayerCharacter.LeftPush` true _player)))

(event `self.Right.OnComponentBeginOverlap`
  (params (OverlappedComponent :type "PrimitiveComponent Object Reference") (OtherActor :type "Actor Object Reference") (OtherComp :type "PrimitiveComponent Object Reference") (OtherBodyIndex :type Integer) (bFromSweep :type Boolean) (SweepResult :type "HitResult Structure (by ref)"))
  (bind _player (`self.Player`))
  (if (== OtherActor _player)
    (set `/Game/Blueprints/BP_PlayerCharacter.LeftPush` false _player)))

(event `self.Box.OnComponentBeginOverlap`
  (params (OverlappedComponent :type "PrimitiveComponent Object Reference") (OtherActor :type "Actor Object Reference") (OtherComp :type "PrimitiveComponent Object Reference") (OtherBodyIndex :type Integer) (bFromSweep :type Boolean) (SweepResult :type "HitResult Structure (by ref)"))
  (if (== OtherActor (`self.Player`))
    (bind _returnvalue (`|CreateWidget` "/Game/UI_UX/Feedback/Tuto/Caisse.Caisse_C"))
    (`UserWidget.AddToViewport` _returnvalue 0)))

(event `self.Box.OnComponentEndOverlap`
  (params (OverlappedComponent :type "PrimitiveComponent Object Reference") (OtherActor :type "Actor Object Reference") (OtherComp :type "PrimitiveComponent Object Reference") (OtherBodyIndex :type Integer))
  (if (== OtherActor (`self.Player`))
    (bind _foundwidgets (`WidgetBlueprintLibrary.GetAllWidgetsOfClass` "/Game/UI_UX/Feedback/Tuto/Caisse.Caisse_C"))
    (bind _ascaisse (cast `/Game/UI_UX/Feedback/Tuto/Caisse` (`|GetArrayItem` _foundwidgets)))
    (`Widget.RemoveFromParent` _ascaisse)))

(fn `UserConstructionScript`)