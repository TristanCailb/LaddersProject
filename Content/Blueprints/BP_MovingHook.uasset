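; BP_MovingHook is an actor that travels to an offset position when something overlaps its Box.
; The PlatformMovement timeline lerps it from its BeginPlay location by the relative EndPoint vector, without sweeping.
; Ending the overlap reverses the timeline after a three-second delay, but only if IsUp is true.
; IsUp is set whenever the timeline finishes, in either direction, and cleared when reversal starts.
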(event `self.ReceiveBeginPlay`
  (set `self.BeginPoint` (`self.K2_GetActorLocation`)))

(event `HookMove`
  (bind (_direction _movement) (`Timeline|PlatformMovement` :!label _label)
    (:`Update`
      (`self.K2_SetActorLocation` (`KismetMathLibrary.VLerp` (`self.BeginPoint`) (+ (`self.BeginPoint`) (`self.EndPoint`)) _movement)))
    (:`Finished`
      (set `self.IsUp` true))))

(event `ReverseMove`
  (set `self.IsUp` false)
  (goto _label :!via `Reverse`))

(event `self.Box.OnComponentBeginOverlap`
  (params (OverlappedComponent :type "PrimitiveComponent Object Reference") (OtherActor :type "Actor Object Reference") (OtherComp :type "PrimitiveComponent Object Reference") (OtherBodyIndex :type Integer) (bFromSweep :type Boolean) (SweepResult :type "HitResult Structure (by ref)"))
  (`self.HookMove`))

(event `self.Box.OnComponentEndOverlap`
  (params (OverlappedComponent :type "PrimitiveComponent Object Reference") (OtherActor :type "Actor Object Reference") (OtherComp :type "PrimitiveComponent Object Reference") (OtherBodyIndex :type Integer))
  (if (`self.IsUp`)
    (`KismetSystemLibrary.Delay` 3.0)
    (`self.ReverseMove`)))

(fn `UserConstructionScript`)