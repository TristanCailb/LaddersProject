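; BP_LadderUpgrade is an actor that marks where the player is allowed to upgrade the ladder.
; On BeginPlay it casts the first player pawn to BP_PlayerCharacter and caches it.
; Its Box overlap events set that player's CanUpgradeLadder flag on entry and clear it on exit, ignoring other actors.
; The upgrade itself is not implemented here, as UpgradeLadderNbChunk is an empty stub.
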(event `self.ReceiveBeginPlay`
  (bind _asbp_player_character (cast `/Game/Blueprints/BP_PlayerCharacter` (`GameplayStatics.GetPlayerPawn` 0)))
  (set `self.Player` _asbp_player_character))

(event `self.Box.OnComponentBeginOverlap`
  (params (OverlappedComponent :type "PrimitiveComponent Object Reference") (OtherActor :type "Actor Object Reference") (OtherComp :type "PrimitiveComponent Object Reference") (OtherBodyIndex :type Integer) (bFromSweep :type Boolean) (SweepResult :type "HitResult Structure (by ref)"))
  (bind _player (`self.Player`))
  (if (== OtherActor _player)
    (set `/Game/Blueprints/BP_PlayerCharacter.CanUpgradeLadder` true _player)))

(event `self.Box.OnComponentEndOverlap`
  (params (OverlappedComponent :type "PrimitiveComponent Object Reference") (OtherActor :type "Actor Object Reference") (OtherComp :type "PrimitiveComponent Object Reference") (OtherBodyIndex :type Integer))
  (bind _player (`self.Player`))
  (if (== OtherActor _player)
    (set `/Game/Blueprints/BP_PlayerCharacter.CanUpgradeLadder` false _player)))

(fn `UpgradeLadderNbChunk`)

(fn `UserConstructionScript`)