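; BP_DronePlat is a platform that moves along a spline when the player enters its trigger box.
; BeginPlay caches the player character, and a box overlap by that actor calls StartMovement.
; StartMovement plays a timeline whose Alpha samples the spline by time to set the platform's relative location.
; A ReverseMovement event can reverse the timeline, but only a disconnected IsUp toggle calls it here.
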(event `self.ReceiveBeginPlay`
  (bind _asbp_player_character (cast `/Game/Blueprints/BP_PlayerCharacter` (`GameplayStatics.GetPlayerPawn` 0)))
  (set `self.Player` _asbp_player_character))

(event `StartMovement`
  (bind (_direction _alpha) (`Timeline|Timeline_0` :!label _label)
    (:`Update`
      (`SceneComponent.K2_SetRelativeLocation` (`self.Platform`) (`SplineComponent.GetLocationAtTime` (`self.Spline`) _alpha "Local" false) false false))))

(event `ReverseMovement`
  (goto _label :!via `Reverse`))

(event `self.Box.OnComponentBeginOverlap`
  (params (OverlappedComponent :type "PrimitiveComponent Object Reference") (OtherActor :type "Actor Object Reference") (OtherComp :type "PrimitiveComponent Object Reference") (OtherBodyIndex :type Integer) (bFromSweep :type Boolean) (SweepResult :type "HitResult Structure (by ref)"))
  (if (== OtherActor (`self.Player`))
    (`self.StartMovement`)))

(fn `UserConstructionScript`)