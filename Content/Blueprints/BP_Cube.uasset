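; BP_Cube is a moving platform whose cube travels along a spline.
; A timeline's Alpha feeds the spline's location-at-time lookup, setting the cube's relative position on each update without sweep.
; The Active event toggles an IsUp flag, playing the timeline forward or reversing it on alternate calls.
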(event `StartMovement`
  (bind (_direction _alpha) (`Timeline|TL_Plateform` :!label _label)
    (:`Update`
      (`SceneComponent.K2_SetRelativeLocation` (`self.Cube`) (`SplineComponent.GetLocationAtTime` (`self.Spline`) _alpha "Local" false) false false))))

(event `ReverseMovement`
  (goto _label :!via `Reverse`))

(event `/Game/Blueprints/BPI_Interuptor.Active`
  (if (`self.IsUp`)
    (`self.ReverseMovement`)
    (set `self.IsUp` false)
    (else
      (`self.StartMovement`)
      (set `self.IsUp` true))))

(fn `UserConstructionScript`)