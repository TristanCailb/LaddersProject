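; BP_LadderFrags is a pickup that adds one ladder fragment to the player.
; BeginPlay casts the first player pawn to BP_PlayerCharacter and caches it.
; When that player overlaps the LadderFrag component, AddFrags increments the character's LadderFrags count and the actor destroys itself.
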(event `self.ReceiveBeginPlay`
  (bind _asbp_player_character (cast `/Game/Blueprints/BP_PlayerCharacter` (`GameplayStatics.GetPlayerPawn` 0)))
  (set `self.Player` _asbp_player_character))

(event `self.LadderFrag.OnComponentBeginOverlap`
  (params (OverlappedComponent :type "PrimitiveComponent Object Reference") (OtherActor :type "Actor Object Reference") (OtherComp :type "PrimitiveComponent Object Reference") (OtherBodyIndex :type Integer) (bFromSweep :type Boolean) (SweepResult :type "HitResult Structure (by ref)"))
  (if (== OtherActor (`self.Player`))
    (`self.AddFrags`)
    (`self.K2_DestroyActor`)))

(fn `AddFrags`
  (bind _player (`self.Player`))
  (set `/Game/Blueprints/BP_PlayerCharacter.LadderFrags` (+ (`/Game/Blueprints/BP_PlayerCharacter.LadderFrags` _player) 1) _player))

(fn `UserConstructionScript`)