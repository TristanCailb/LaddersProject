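; Portable ladder actor that the player carries on their back, holds in hands or drops on the ground to climb.
; SetLadderState switches visibility, physics and collision per state, showing the player's own ladder component while stowed.
; CanClimb requires a grounded ladder within a 45-degree slope pitch limit, and is pushed to the player on trigger overlap or drop.
; UpgradeLadder is an unfinished stub.
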(event `self.ReceiveBeginPlay`
  ;[1 1 1] Set the starting ladder state
  (`self.SetLadderState` (`self.LadderState`))
  (bind _asbp_player_character (cast `/Game/Blueprints/BP_PlayerCharacter` (`self.Instigator`)))
  (set `self.Player` _asbp_player_character))

(event `self.Trigger.OnComponentBeginOverlap`
  (params (OverlappedComponent :type "PrimitiveComponent Object Reference") (OtherActor :type "Actor Object Reference") (OtherComp :type "PrimitiveComponent Object Reference") (OtherBodyIndex :type Integer) (bFromSweep :type Boolean) (SweepResult :type "HitResult Structure (by ref)"))
  ;[1 1 1] Player enter trigger
  (if (`self.IsOnTheGround`)
    (if (== OtherActor (`self.Player`))
      (set `/Game/Blueprints/BP_PlayerCharacter.CanClimb` (`self.CanClimb`) (`self.Player`)))))

(event `self.Trigger.OnComponentEndOverlap`
  (params (OverlappedComponent :type "PrimitiveComponent Object Reference") (OtherActor :type "Actor Object Reference") (OtherComp :type "PrimitiveComponent Object Reference") (OtherBodyIndex :type Integer))
  ;[1 1 1] Player leave trigger
  (if (== OtherActor (`self.Player`))
    (set `/Game/Blueprints/BP_PlayerCharacter.CanClimb` false (`self.Player`))))

(fn `CanClimb`
  (returns (Value :type Boolean))
  (bind _outslopepitchdegreeangle (`KismetMathLibrary.GetSlopeDegreeAngles` (`self.GetActorRightVector`) (`KismetMathLibrary.MakeVector` 0.0 0.0 1.0) (`self.GetActorUpVector`)))
  ;[1 1 1] Check if the player can climb
  (return (and (`|EnumEquality` (`self.LadderState`) "NewEnumerator2") (and (> _outslopepitchdegreeangle -45.0) (< _outslopepitchdegreeangle 45.0)))))

(fn `IsInHands`
  (returns (Value :type Boolean))
  ;[1 1 1] If the ladder is on the ground
  (return (`|EnumEquality` (`self.LadderState`) "NewEnumerator1")))

(fn `IsOnTheGround`
  (returns (Value :type Boolean))
  ;[1 1 1] If the ladder is on the ground
  (return (`|EnumEquality` (`self.LadderState`) "NewEnumerator2")))

(fn `SetLadderMeshCollision`
  (params (Collision :type "ECollisionEnabled Enum" :default "NoCollision"))
  ;[1 1 1] Update ladder collisions
  (if (`self.CanClimb`)
    (`PrimitiveComponent.SetCollisionEnabled` (`self.StaticMesh`) Collision)))

(fn `SetLadderState`
  (params (State :type "/Game/Blueprints/Ladder/E_LadderState Enum" :default "NewEnumerator0"))
  (bind _staticmesh (`self.StaticMesh`))
  (bind _staticmesh_2 (`self.StaticMesh`))
  (bind _staticmesh_3 (`self.StaticMesh`))
  ;[1 1 1] Set ladder state and update collisions
  (bind _asbp_player_character (cast `/Game/Blueprints/BP_PlayerCharacter` (`GameplayStatics.GetPlayerPawn` 0)))
  (bind _output_get (set `self.LadderState` State))
  (switch `/Game/Blueprints/Ladder/E_LadderState` _output_get
    (:`NewEnumerator0`
      (bind _echelle (`/Game/Blueprints/BP_PlayerCharacter.Echelle` _asbp_player_character))
      (`SceneComponent.SetVisibility` _echelle true false)
      (`self.SetActorHiddenInGame` true)
      (`PrimitiveComponent.SetSimulatePhysics` _staticmesh_2 false)
      (`PrimitiveComponent.SetCollisionEnabled` _staticmesh_2 "NoCollision")
      (`self.SetLadderMeshCollision` "NoCollision"))
    (:`NewEnumerator1`
      (`SceneComponent.SetVisibility` _echelle false false)
      (`self.SetActorHiddenInGame` false)
      (`PrimitiveComponent.SetSimulatePhysics` _staticmesh_3 true)
      (`PrimitiveComponent.SetCollisionEnabled` _staticmesh_3 "QueryAndPhysics")
      (`self.SetLadderMeshCollision` "QueryAndPhysics"))
    (:`NewEnumerator2`
      (`SceneComponent.SetVisibility` _echelle false false)
      (`self.SetActorHiddenInGame` false)
      (`PrimitiveComponent.SetSimulatePhysics` _staticmesh true)
      (`PrimitiveComponent.SetCollisionEnabled` _staticmesh "QueryAndPhysics")
      (`self.SetLadderMeshCollision` "QueryAndPhysics")
      ;[1 1 1] Check if the player can climb when he drops the ladder
      (bind _asbp_player_character_2 (cast `/Game/Blueprints/BP_PlayerCharacter` (`self.Instigator`)))
      (set `/Game/Blueprints/BP_PlayerCharacter.CanClimb` (`self.CanClimb`) _asbp_player_character_2))))

(fn `UpgradeLadder`)

(fn `UserConstructionScript`)